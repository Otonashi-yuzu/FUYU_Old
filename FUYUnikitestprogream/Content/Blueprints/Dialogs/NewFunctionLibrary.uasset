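; Dialog helper function library for raising a character memory value and showing character icon widgets.
; Wordgoodchoise and Goodchoise identically add a fixed amount to the stored memory value.
; Icon and Iconout each construct a new BP_chactericon for a given row name, add it to the viewport and play a slowed in or out animation.
; Iconout removes no existing widget, and the two NewFunction stubs are empty.
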(fn Wordgoodchoise
  (|CharacterMemorySetNode (+ 5.0 (|CharacterMemoryGetNode))))

(fn NewFunction)

(fn Icon
  (params (NewParam :type Boolean%20%28by%20ref%29) (Row%20Name :type Name) (Outer :type Object%20Object%20Reference))
  (bind _returnvalue (Game|ConstructObjectfromClass Outer "/Game/Blueprints/UI/ingame/BP_chactericon.BP_chactericon_C" Row%20Name))
  (UserInterface|Viewport|AddtoViewport _returnvalue 0)
  (UserInterface|Animation|PlayAnimation _returnvalue (Variables|/Game/Blueprints/UI/ingame/BP_chactericon.BP_chactericon_C|Getanimation_in _returnvalue) 0.0 1 "PingPong" 0.2 false))

(fn Iconout
  (params (目标 :type BP%20Chactericon%20Object%20Reference) (目标1 :type User%20Widget%20Object%20Reference) (Row%20Name :type Name))
  (bind _returnvalue (Game|ConstructObjectfromClass 目标 "/Game/Blueprints/UI/ingame/BP_chactericon.BP_chactericon_C" Row%20Name))
  (UserInterface|Viewport|AddtoViewport _returnvalue 0)
  (UserInterface|Animation|PlayAnimation _returnvalue (Variables|/Game/Blueprints/UI/ingame/BP_chactericon.BP_chactericon_C|Getout _returnvalue) 0.0 1 "Forward" 0.1 false))

(fn Goodchoise
  (|CharacterMemorySetNode (+ 5.0 (|CharacterMemoryGetNode))))

(fn NewFunction0)