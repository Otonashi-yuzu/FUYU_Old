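; Backpack (beibao) inventory Blueprint that stores picked-up item records in the Baoneiwupin array.
; Huoquwupin adds an item; Shiyong branches on item type, then removes the used item.
; Keys write their panduan value to character memory, while medicine adds its xiaoguo effect to the stored character value.
; Open (Dakaibeibao) and discard (Diuqi) are empty stubs, with unconnected ItemInfo lookup and widget-creation nodes left over.
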(event EventBeginPlay)

(event EventTick
  (params (DeltaSeconds :type Float%20%28single-precision%29)))

(fn Dakaibeibao)

(fn Huoquwupin
  (params (wupinxinxi :type Wupinxinxi%20Structure))
  (Utilities|Array|Add (Variables|Default|Getbaoneiwupin) wupinxinxi))

(fn Shiyong
  (params (wupinxinxi :type Wupinxinxi%20Structure))
  (bind _output_get (LocalVariables|Setwupinzancun wupinxinxi))
  (Utilities|FlowControl|Sequence
    (:then_0
      (switch Utilities|FlowControl|Switch|Switchonwupinfenlei (.类型 (Utilities|Struct|Breakwupinxinxi _output_get))
        (:NewEnumerator0
          ;[1 1 1] 钥匙
          (|CharacterMemorySetNode (.panduan (LocalVariables|Getwupinzancun))))
        (:NewEnumerator1
          ;[1 1 1] 药物
          (|CharacterMemorySetNode (+ (.xiaoguo (LocalVariables|Getwupinzancun)) (|CharacterMemoryGetNode))))))
    (:then_1
      (Utilities|Array|RemoveItem (Variables|Default|Getbaoneiwupin) (LocalVariables|Getwupinzancun)))))

(fn Diuqi)