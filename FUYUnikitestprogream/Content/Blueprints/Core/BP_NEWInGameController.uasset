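; In-game player controller for a dialogue-driven game, mapping input to dialogue, save/load, pause and backpack UI.
; Touch or NextDialog advances the HUD's DialogControllerComponent unless the pause menu is visible; mouse wheel down rolls back a snapshot.
; AUTIO toggles auto-advance, which runs from Tick through a short Delay and bypasses that visibility check.
; Save and load capture a screenshot, then open their pages in a reused or lazily created pause menu.
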(event Custom|ShowPauseWidget
  (Class|GameSaveSubsystem|ClearLoadingFlag (Subsystems|GetGameSaveSubsystem))
  (bind _pausemenu (CallFunction|GetPauseMenuWidget))
  (Widget|SetVisibility _pausemenu "Visible"))

(event Custom|ShowLoadGameWidget
  (Class|GameSaveSubsystem|CreateScreenShotforSaveGame (Subsystems|GetGameSaveSubsystem))
  (bind _pausemenu (CallFunction|GetPauseMenuWidget))
  (Widget|SetVisibility _pausemenu "Visible")
  (Class|PauseMenuWidget|GotoLoadGameWidget _pausemenu))

(event Custom|AUTIO
  (bind _isa (Utilities|FlowControl|FlipFlop)
    (:A
      _)
    (:B
      _))
  (Variables|Default|Setauto _isa))

(event Custom|ShowSaveGameWidget
  (Class|GameSaveSubsystem|CreateScreenShotforSaveGame (Subsystems|GetGameSaveSubsystem))
  (bind _pausemenu (CallFunction|GetPauseMenuWidget))
  (Widget|SetVisibility _pausemenu "Visible")
  (Class|PauseMenuWidget|GotoSaveGameWidget _pausemenu))

(event EventTick
  (params (DeltaSeconds :type Float%20%28single-precision%29))
  (if (Variables|Default|Getauto)
    (Utilities|FlowControl|Delay 0.2)
    (Class|DialogControllerComponent|MovetoNextDialog (Actor|GetComponentbyClass (HUD|GetHUD) "/Script/VNM.DialogControllerComponent"))))

(event Input|ActionEvents|InputActionNextDialog
  (params (Key :type Key%20Structure :default "None"))
  (bind _returnvalue (HUD|GetHUD))
  (bind _returnvalue_2 (Actor|GetComponentbyClass _returnvalue "/Script/VNM.DialogControllerComponent"))
  (:Pressed
    (Utilities|IsValid _returnvalue_2
      (:Is%20Valid
        (bind _pausemenu (CallFunction|GetPauseMenuWidget))
        (if (not (Widget|IsVisible _pausemenu))
          (Class|DialogControllerComponent|MovetoNextDialog _returnvalue_2))))))

(event Input|ActionEvents|InputActionSaveGame
  (params (Key :type Key%20Structure :default "None"))
  (:Pressed
    (CallFunction|ShowSaveGameWidget)))

(event Input|ActionEvents|InputActionLoadGame
  (params (Key :type Key%20Structure :default "None"))
  (:Pressed
    (CallFunction|ShowLoadGameWidget)))

(event Input|ActionEvents|InputActionReturnToMainMenu
  (params (Key :type Key%20Structure :default "None"))
  (:Pressed
    (CallFunction|ShowPauseWidget)))

(event Input|MouseEvents|MouseWheelDown
  (params (Key :type Key%20Structure :default "None"))
  (bind _returnvalue (HUD|GetHUD))
  (bind _returnvalue_2 (Actor|GetComponentbyClass _returnvalue "/Script/VNM.DialogRollbackControllerComponent"))
  (:Pressed
    (Utilities|IsValid _returnvalue_2
      (:Is%20Valid
        (Class|DialogRollbackControllerComponent|RollbackOneSnapshot _returnvalue_2)))))

(event Input|KeyboardEvents|B
  (params (Key :type Key%20Structure :default "None"))
  (:Pressed
    (bind _returnvalue (Game|ConstructObjectfromClass "/Game/Blueprints/UI/ingame/beibao/beibaozhuUI.beibaozhuUI_C" (Variables|Default|Getbeibao)))
    (UserInterface|Animation|PlayAnimation _returnvalue 0 0.0 1 "Forward" 1.0 false)
    (UserInterface|Viewport|AddtoViewport _returnvalue 0)))

(event Input|TouchEvents|InputTouch
  (params (Location :type Vector) (FingerIndex :type ETouchIndex%20Enum))
  (bind _returnvalue (HUD|GetHUD))
  (bind _returnvalue_2 (Actor|GetComponentbyClass _returnvalue "/Script/VNM.DialogControllerComponent"))
  (:Pressed
    (Utilities|IsValid _returnvalue_2
      (:Is%20Valid
        (bind _pausemenu (CallFunction|GetPauseMenuWidget))
        (if (not (Widget|IsVisible _pausemenu))
          (Class|DialogControllerComponent|MovetoNextDialog _returnvalue_2))))))

(fn ConstructionScript)

(fn GetPauseMenuWidget
  (bind _foundwidgets (Widget|GetAllWidgetsOfClass "/VisualNovelMachinery/Blueprints/UI/MainMenu/W_PauseMenuWidget.W_PauseMenuWidget_C" false))
  (bind _output_get (LocalVariables|SetPauseMenus _foundwidgets))
  (if (== (Utilities|Array|Length _output_get) 1)
    (return (Utilities|Array|Get(acopy) (LocalVariables|GetPauseMenus)))
    (else
      (bind _returnvalue (UserInterface|CreateWidget "/VisualNovelMachinery/Blueprints/UI/MainMenu/W_PauseMenuWidget.W_PauseMenuWidget_C" self))
      (UserInterface|Viewport|AddtoViewport _returnvalue 0)
      (Widget|SetVisibility _returnvalue "Collapsed")
      (return _returnvalue))))